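; Base VR option actor that displays one selectable color, pattern, decal, mesh or teleporter choice, spawned as a child actor of OptionHandler_BP.
; The handler supplies type, UI style and info, which drive dynamic materials and text.
; When projected, Tick fades it in and, while ungrabbed, interpolates roll and a touch-based forward offset.
; ActivateOption applies the choice to the handler's owning ArchVisVR actor, or teleports the owning pawn by option index.
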(event `self.ReceiveTick`
  (params (DeltaSeconds :type "Float (single-precision)"))
  (bind _returnvalue (`self.K2_GetActorLocation`))
  (bind _roll (.roll (`self.K2_GetActorRotation`)))
  (bind _returnvalue_2 (`KismetMathLibrary.SelectVector` (+ (`self.DesiredLocation`) (* (`SceneComponent.GetForwardVector` (`self.Forward`)) 15.0)) (`self.DesiredLocation`) (`self.bTouched`)))
  ;[1 1 1] Option movement and animtion depends on active or not
  (if (`self.bProjected`)
    (`|ExecutionSequence`
      (:`then_0`
        (if (`self.bGrabed`)
          ;;[1 1 1] Selected
          (set `self.DesiredLocation` (`self.K2_GetActorLocation`))
          (set `self.DesiredRotation` (`self.K2_GetActorRotation`))
          (`/Engine/EditorBlueprintResources/StandardMacros.DoOnce` false :!label _label
            (:`Completed`
              (if (`self.bTouched`)
                (`self.K2_SetActorLocation` (+ (`self.DesiredLocation`) (* (`SceneComponent.GetForwardVector` (`self.Forward`)) -15.0)) false true))))
          (else
            ;;[1 1 1] set Rotation
            (`|ExecutionSequence`
              (:`then_0`
                (if (!= _roll (`self.DesiredDegree`))
                  (bind _output_get (set `self.DesiredRotation` (`KismetMathLibrary.MakeRotator` (`KismetMathLibrary.FInterpTo` _roll (`self.DesiredDegree`) DeltaSeconds 2.0) (.pitch (`self.K2_GetActorRotation`)) (.yaw (`self.K2_GetActorRotation`)))))
                  (`self.K2_SetActorRotation` _output_get)))
              (:`then_1`
                ;;[1 1 1] Set location when it's not selected
                (if (!= _returnvalue _returnvalue_2 :`ErrorTolerance` 0.1)
                  (`self.K2_SetActorLocation` (`KismetMathLibrary.VInterpTo` _returnvalue _returnvalue_2 DeltaSeconds 8.0) false true)
                  (goto _label :!via `Reset`)))))))
      (:`then_1`
        ;[1 1 1] Animate opacity
        (`/Engine/EditorBlueprintResources/StandardMacros.DoOnce` false
          (:`Completed`
            (bind (_direction _opacity) (`Timeline|OpeningEffect` :!via `PlayFromStart`)
              (:`Update`
                (`MaterialInstanceDynamic.SetScalarParameterValue` (`self.MID_1`) "GlobalOpacity" _opacity)
                (`MaterialInstanceDynamic.SetScalarParameterValue` (`self.CurrentMaterial`) "GlobalOpacity" (* _opacity 5.0))))))))))

(fn `ActivateOption`
  (bind _asoption_handler_bp (cast `/Game/ArchVisVR/Blueprints/Option/OptionHandler_BP` (`self.GetParentActor`)))
  (bind _returnvalue (`self.GetOwner` _asoption_handler_bp))
  (bind _asarch_vis_vr_base_actor_bp (cast `/Game/ArchVisVR/Blueprints/Actor/ArchVisVR_BaseActor_BP` _returnvalue)
    (:`then`
      (`GameplayStatics.PlaySound2D` (`self.SoundToPlay`) 1.0 1.0 0.0 null null)
      (switch `/Game/ArchVisVR/Blueprints/Option/OptionType/ArchVisVR_Options` (`self.OptionType`)
        (:`NewEnumerator0`
          (`/Game/ArchVisVR/Blueprints/Actor/ArchVisVR_BaseActor_BP.ApplyNewColor` _asarch_vis_vr_base_actor_bp (`self.ColorInfo`)))
        (:`NewEnumerator1`
          (`/Game/ArchVisVR/Blueprints/Actor/ArchVisVR_BaseActor_BP.ApplyNewPattern` _asarch_vis_vr_base_actor_bp (`self.PatternInfo`)))
        (:`NewEnumerator2`
          (`/Game/ArchVisVR/Blueprints/Actor/ArchVisVR_BaseActor_BP.ApplyNewDecal` _asarch_vis_vr_base_actor_bp (`self.DecalInfo`)))
        (:`NewEnumerator3`
          (`/Game/ArchVisVR/Blueprints/Actor/ArchVisVR_BaseActor_BP.ApplyNewMesh` _asarch_vis_vr_base_actor_bp (`self.MeshInfo`)))))
    (:`CastFailed`
      (bind _asarch_vis_vrpawn_bp (cast `/Game/ArchVisVR/Blueprints/Player/ArchVis_VRPawn_BP` _returnvalue))
      (switch `/Game/ArchVisVR/Blueprints/Option/OptionType/ArchVisVR_Options` (`self.OptionType`)
        (:`NewEnumerator5`
          (for (_array_element _array_index) (`/Game/ArchVisVR/Blueprints/Option/OptionHandler_BP.Options` _asoption_handler_bp)
            (if (== (`ChildActorComponent.ChildActor` _array_element) self)
              (`/Game/ArchVisVR/Blueprints/Player/ArchVis_VRPawn_BP.TeleportTo` _asarch_vis_vrpawn_bp _array_index)
              (break))))))))

(fn `OptionToShow`
  (params (NewColorInfo :type "/Game/ArchVisVR/Blueprints/Option/OptionType/ArchVisVR_ColorOption Structure") (NewPatternInfo :type "/Game/ArchVisVR/Blueprints/Option/OptionType/ArchVisVR_PatternOption Structure") (NewDecalInfo :type "/Game/ArchVisVR/Blueprints/Option/OptionType/ArchVisVR_DecalOption Structure") (NewMeshInfo :type "/Game/ArchVisVR/Blueprints/Option/OptionType/ArchVisVR_MeshOption Structure") (NewTeleporterInfo :type "/Game/ArchVisVR/Blueprints/Option/OptionType/ArchVisVR_TeleporterOption Structure"))
  (switch `/Game/ArchVisVR/Blueprints/Option/OptionType/ArchVisVR_Options` (`self.OptionType`)
    (:`NewEnumerator0`
      ;[1 1 1] Set colors info from handler
      (bind _output_get (set `self.ColorInfo` NewColorInfo))
      (bind (_color _meshindex _name _fontsize) (break `/Game/ArchVisVR/Blueprints/Option/OptionType/ArchVisVR_ColorOption` _output_get))
      (`MaterialInstanceDynamic.SetVectorParameterValue` (`self.CurrentMaterial`) "Color" _color)
      (`TextRenderComponent.K2_SetText` (`self.OptionText`) _name)
      (`TextRenderComponent.SetWorldSize` (`self.OptionText`) _fontsize))
    (:`NewEnumerator1`
      ;[1 1 1] Set patterns info from handler
      (bind _output_get_2 (set `self.PatternInfo` NewPatternInfo))
      (bind (_basetexture _patternmaterialinstance _meshindex_2 _name_2 _fontsize_2) (break `/Game/ArchVisVR/Blueprints/Option/OptionType/ArchVisVR_PatternOption` _output_get_2))
      (`MaterialInstanceDynamic.SetTextureParameterValue` (`self.CurrentMaterial`) "BaseTexture" _basetexture)
      (`TextRenderComponent.K2_SetText` (`self.OptionText`) _name_2)
      (`TextRenderComponent.SetWorldSize` (`self.OptionText`) _fontsize_2))
    (:`NewEnumerator2`
      ;[1 1 1] Set decal info from handler
      (bind _output_get_3 (set `self.DecalInfo` NewDecalInfo))
      (bind (_decalbasetexture _decalmaterialinstance _minsize _maxsize _name_3 _fontsize_3) (break `/Game/ArchVisVR/Blueprints/Option/OptionType/ArchVisVR_DecalOption` _output_get_3))
      (`MaterialInstanceDynamic.SetTextureParameterValue` (`self.CurrentMaterial`) "BaseTexture" _decalbasetexture)
      (`TextRenderComponent.K2_SetText` (`self.OptionText`) _name_3)
      (`TextRenderComponent.SetWorldSize` (`self.OptionText`) _fontsize_3))
    (:`NewEnumerator3`
      ;[1 1 1] Set mesh info from handler
      (bind _output_get_4 (set `self.MeshInfo` NewMeshInfo))
      (bind (_picture _mesh _meshtransofrm _text _fontsize_4) (break `/Game/ArchVisVR/Blueprints/Option/OptionType/ArchVisVR_MeshOption` _output_get_4))
      (`MaterialInstanceDynamic.SetTextureParameterValue` (`self.CurrentMaterial`) "BaseTexture" _picture)
      (`TextRenderComponent.K2_SetText` (`self.OptionText`) _text)
      (`TextRenderComponent.SetWorldSize` (`self.OptionText`) _fontsize_4))
    (:`NewEnumerator5`
      ;[1 1 1] Set Teleporter info for handler
      (bind _output_get_5 (set `self.TeleporterInfo` NewTeleporterInfo))
      (bind (_picture_2 _mesh_2 _transform _text_2 _fontsize_5) (break `/Game/ArchVisVR/Blueprints/Option/OptionType/ArchVisVR_TeleporterOption` _output_get_5))
      (`MaterialInstanceDynamic.SetTextureParameterValue` (`self.CurrentMaterial`) "BaseTexture" _picture_2)
      (`TextRenderComponent.K2_SetText` (`self.OptionText`) _text_2)
      (`TextRenderComponent.SetWorldSize` (`self.OptionText`) _fontsize_5))))

(fn `SetOptionType`
  (params (NewType :type "/Game/ArchVisVR/Blueprints/Option/OptionType/ArchVisVR_Options Enum" :default "NewEnumerator0"))
  (bind _optionmesh (`self.OptionMesh`))
  ;[1 1 1] Set option type from handler
  (bind _output_get (set `self.OptionType` NewType))
  ;[1 1 1] Create material instance to show option
  (switch `/Game/ArchVisVR/Blueprints/Option/OptionType/ArchVisVR_Options` _output_get
    (:`NewEnumerator0`
      (bind _returnvalue (`PrimitiveComponent.CreateDynamicMaterialInstance` _optionmesh 1 "/Game/ArchVisVR/Materials/Option/MI_Option_BaseNoTexture.MI_Option_BaseNoTexture" "None"))
      (set `self.CurrentMaterial` _returnvalue))
    (:`NewEnumerator1`
      (bind _returnvalue_2 (`PrimitiveComponent.CreateDynamicMaterialInstance` _optionmesh 1 "/Game/ArchVisVR/Materials/Option/MI_Option_BaseTextured.MI_Option_BaseTextured" "None" :!label _label))
      (set `self.CurrentMaterial` _returnvalue_2))
    (:`NewEnumerator2`
      (goto _label))
    (:`NewEnumerator3`
      (goto _label))
    (:`NewEnumerator5`
      (goto _label)))
  (`MaterialInstanceDynamic.SetScalarParameterValue` (`self.CurrentMaterial`) "GlobalOpacity" 0.0))

(fn `SetUIStyle`
  (params (NewUI :type "/Game/ArchVisVR/Blueprints/Option/OptionType/ArchVisVR_UIStyle Structure"))
  (bind (_mesh _textoffset) (break `/Game/ArchVisVR/Blueprints/Option/OptionType/ArchVisVR_UIStyle` NewUI))
  (bind _optionmesh (`self.OptionMesh`))
  (`StaticMeshComponent.SetStaticMesh` (`self.OptionMesh`) _mesh)
  (`SceneComponent.K2_AddLocalOffset` (`self.OptionText`) _textoffset false false)
  (bind _returnvalue (`PrimitiveComponent.CreateDynamicMaterialInstance` _optionmesh 0 (`|GetArrayItem` (`MeshComponent.GetMaterials` _optionmesh)) "None"))
  (bind _output_get (set `self.MID_1` _returnvalue))
  (`MaterialInstanceDynamic.SetScalarParameterValue` _output_get "GlobalOpacity" 0.0))

(fn `UserConstructionScript`)