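; VR light switch actor for ArchVis that toggles a set of lights and emissive meshes when touched by a motion controller's pointer sphere.
; The overlap flips On, then ToggleSwitch tilts the switch, lights its LED only when off, and sets each LightsInfo light's intensity.
; SetBrightnessOnMesh drives paired mesh materials through dynamic instances.
; The construction script runs the same toggle logic to apply the initial On state.
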(event `self.Switch_Collision.OnComponentBeginOverlap`
  (params (OverlappedComponent :type "PrimitiveComponent Object Reference") (OtherActor :type "Actor Object Reference") (OtherComp :type "PrimitiveComponent Object Reference") (OtherBodyIndex :type Integer) (bFromSweep :type Boolean) (SweepResult :type "HitResult Structure (by ref)"))
  ;[1 1 1] Switch the light
  (bind _asarch_vis_motion_controller_bp (cast `/Game/ArchVisVR/Blueprints/Player/ArchVis_MotionController_BP` OtherActor))
  (if (== (`/Game/ArchVisVR/Blueprints/Player/ArchVis_MotionController_BP.PointerSphere` _asarch_vis_motion_controller_bp) OtherComp)
    (set `self.bOn` (not (`self.bOn`)))
    (`self.ToggleSwitch`)))

(fn `SetBrightnessOnMesh`
  (for _array_element (`self.LightsInfo`)
    (bind (_light _intensity _mesh _meshindex _materialbrightness _materialparametername) (break `/Game/ArchVisVR/Blueprints/Option/OptionType/ArchVisVR_LightOptions` _array_element))
    (`/Engine/EditorBlueprintResources/StandardMacros.IsValid` _mesh
      (:`Is Valid`
        (bind _staticmeshcomponent (`StaticMeshActor.StaticMeshComponent` _mesh))
        (bind _returnvalue (`PrimitiveComponent.CreateDynamicMaterialInstance` _staticmeshcomponent _meshindex (`PrimitiveComponent.GetMaterial` _staticmeshcomponent _meshindex) "None"))
        (`MaterialInstanceDynamic.SetScalarParameterValue` _returnvalue _materialparametername (`KismetMathLibrary.SelectFloat` _materialbrightness 0.0 (`self.bOn`)))))))

(fn `ToggleSwitch`
  ;[1 1 1] Change rotation on switch
  (`SceneComponent.K2_SetRelativeRotation` (`self.Switch`) (`KismetMathLibrary.SelectRotator` (struct :`Roll` 5.0) (struct :`Roll` -5.0) (`self.bOn`)) false false)
  ;[1 1 1] Set brightness for LED on switch
  (bind _returnvalue (`PrimitiveComponent.CreateDynamicMaterialInstance` (`self.LED`) 0 null "None"))
  (`MaterialInstanceDynamic.SetScalarParameterValue` _returnvalue "Brightness" (`KismetMathLibrary.SelectFloat` 0.0 1.0 (`self.bOn`)))
  ;[1 1 1] Set light brightness for all related lights
  (for _array_element (`self.LightsInfo`)
    (bind (_light _intensity) (break `/Game/ArchVisVR/Blueprints/Option/OptionType/ArchVisVR_LightOptions` _array_element))
    (`/Engine/EditorBlueprintResources/StandardMacros.IsValid` _light
      (:`Is Valid`
        (`LightComponent.SetIntensity` (`Light.LightComponent` _light) (`KismetMathLibrary.SelectFloat` _intensity 0.0 (`self.bOn`))))))
  (`self.SetBrightnessOnMesh`))

(fn `UserConstructionScript`
  (`self.ToggleSwitch`))