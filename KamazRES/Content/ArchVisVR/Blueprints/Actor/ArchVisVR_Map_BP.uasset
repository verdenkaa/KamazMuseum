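; Map actor for ArchVis VR that defines a building's floors, each with a floor plan and teleporter locations.
; The construction script rebuilds one stacked, scaled mesh per floor at cumulative heights, feeding each plan texture into a dynamic material and optionally hiding it.
; GetCurrentFloorInfo finds the player's floor by comparing VR camera height from the top floor down.
; GetAllMainTeleporters gathers the first main teleporter of each floor.
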(fn `GetAllMainTeleporters`
  (returns (NewTeleporters :type "Array of /Game/ArchVisVR/Blueprints/Actor/ArchVisVR_Teleporter Object Reference"))
  (locals (MainTeleports :type "Array of /Game/ArchVisVR/Blueprints/Actor/ArchVisVR_Teleporter Object Reference"))
  (for _array_element (`self.Floors`)
    (for _array_element_2 (`.TeleporterLocations_12_E99E3C9648A24B9C76BAE2938D4C0A13` (break `/Game/ArchVisVR/Blueprints/Option/OptionType/ArchVisVR_FloorOption` _array_element))
      (bind (_teleporteroptions_picture _teleporteroptions_mesh _teleporteroptions_transform _teleporteroptions_text _teleporteroptions_fontsize _teleporteroptions_bmainfloorteleporter) (break `/Game/ArchVisVR/Blueprints/Option/OptionType/ArchVisVR_TeleporterOption` (`/Game/ArchVisVR/Blueprints/Actor/ArchVisVR_Teleporter.TeleporterOptions` _array_element_2)))
      (if _teleporteroptions_bmainfloorteleporter
        (`KismetArrayLibrary.Array_Add` (`local.MainTeleports`) _array_element_2)
        (break))))
  (return (`local.MainTeleports`)))

(fn `GetCurrentFloorInfo`
  (returns (FloorInfo :type "/Game/ArchVisVR/Blueprints/Option/OptionType/ArchVisVR_FloorOption Structure"))
  (locals (TempFloorInfo :type "/Game/ArchVisVR/Blueprints/Option/OptionType/ArchVisVR_FloorOption Structure") (bFound :type Boolean) (Index :type Integer) (TempHeight :type "Float (double-precision)" :default 0.0))
  (bind _floors (`self.Floors`))
  (bind _returnvalue (`KismetArrayLibrary.Array_Length` _floors))
  (bind _output (`|GetArrayItem` (`self.Floors`) (`local.Index`)))
  (bind _asarch_vis_vrpawn_bp (cast `/Game/ArchVisVR/Blueprints/Player/ArchVis_VRPawn_BP` (`GameplayStatics.GetPlayerPawn` 0))
    (:`then`
      (if (> _returnvalue 1)
        (set `local.TempHeight` (`self.CurrentHeight`))
        (set `local.Index` (- _returnvalue 1))
        (while (and (not (`local.bFound`)) (>= (`local.Index`) 0))
          (bind (_returnvalue_x _returnvalue_y _returnvalue_z) (`KismetMathLibrary.BreakVector` (`SceneComponent.K2_GetComponentLocation` (`/Game/ArchVisVR/Blueprints/Player/ArchVis_VRPawn_BP.Camera` _asarch_vis_vrpawn_bp))))
          (if (>= _returnvalue_z (`local.TempHeight`))
            (set `local.TempFloorInfo` _output)
            (set `local.Index` 0)
            (set `local.bFound` true)
            (return (`local.TempFloorInfo`))
            (else
              (set `local.TempHeight` (- (`local.TempHeight`) (`.FloorHeight_30_223129CA473637A807A21287C1540AD4` (break `/Game/ArchVisVR/Blueprints/Option/OptionType/ArchVisVR_FloorOption` _output))))
              (set `local.Index` (- (`local.Index`) 1)))))
        (else
          (set `local.TempFloorInfo` (`|GetArrayItem` _floors))
          (return (`local.TempFloorInfo`)))))
    (:`CastFailed`
      (return (`local.TempFloorInfo`)))))

(fn `UserConstructionScript`
  (locals (TempMesh :type "StaticMeshComponent Object Reference"))
  (bind (_returnvalue_x _returnvalue_y _returnvalue_z) (`KismetMathLibrary.BreakVector` (`self.K2_GetActorLocation`)))
  (bind _floors (`self.Floors`))
  ;[1 1 1] Clear existing floors
  (for _array_element (`self.FloorMeshes`)
    (`ActorComponent.K2_DestroyComponent` _array_element))
  (`KismetArrayLibrary.Array_Clear` (`self.FloorMeshes`))
  (set `self.CurrentHeight` _returnvalue_z)
  (for (_array_element_2 _array_index) (`self.Floors`)
    (if (> _array_index 0)
      (bind (_floorplan _teleporterlocations _floorscale _floorheight _hidemapmesh) (break `/Game/ArchVisVR/Blueprints/Option/OptionType/ArchVisVR_FloorOption` _array_element_2))
      (bind _returnvalue (+ _floorheight (`self.CurrentHeight`)))
      (bind (_output_floorplan _output_teleporterlocations _output_floorscale _output_floorheight) (break `/Game/ArchVisVR/Blueprints/Option/OptionType/ArchVisVR_FloorOption` (`|GetArrayItem` _floors (- _array_index 1))))
      ;[1 1 1] Try to make floors height in order
      (if (not (> _returnvalue _output_floorheight))
        (bind (_output_floorplan_2 _output_teleporterlocations_2 _output_floorscale_2 _output_floorheight_2 _output_hidemapmesh) (break `/Game/ArchVisVR/Blueprints/Option/OptionType/ArchVisVR_FloorOption` (`|GetArrayItem` _floors _array_index)))
        (`KismetArrayLibrary.Array_Set` (`self.Floors`) _array_index (make `/Game/ArchVisVR/Blueprints/Option/OptionType/ArchVisVR_FloorOption` _output_floorplan_2 _output_teleporterlocations_2 _output_floorscale_2 0.0 _output_hidemapmesh))))
    (bind _returnvalue_2 (* _floorscale 1.0))
    (bind _returnvalue_3 (`AddComponent|NODE_AddStaticMeshComponent-0` :`bManualAttachment` true :`RelativeTransform` (`KismetMathLibrary.MakeTransform` (`KismetMathLibrary.MakeVector` (.x (.location (`self.GetTransform`))) (.y (.location (`self.GetTransform`))) _returnvalue) (.rotation (`self.GetTransform`)) (`KismetMathLibrary.MakeVector` _returnvalue_2 _returnvalue_2 1.0))))
    (bind _output_get (set `local.TempMesh` _returnvalue_3))
    (bind _returnvalue_4 (`PrimitiveComponent.CreateDynamicMaterialInstance` _output_get 0 (`PrimitiveComponent.GetMaterial` _returnvalue_3 0) "None"))
    (`MaterialInstanceDynamic.SetTextureParameterValue` _returnvalue_4 "FloorMap" _floorplan)
    (`PrimitiveComponent.SetMaterial` (`local.TempMesh`) 0 _returnvalue_4)
    (`SceneComponent.SetVisibility` (`local.TempMesh`) (not _hidemapmesh) false)
    (set `self.CurrentHeight` _returnvalue)
    (`KismetArrayLibrary.Array_Add` (`self.FloorMeshes`) (`local.TempMesh`))))