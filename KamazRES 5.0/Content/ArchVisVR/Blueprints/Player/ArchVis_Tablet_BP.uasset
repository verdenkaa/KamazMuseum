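; VR tablet for architectural visualization that can be picked up and dropped, showing a floor map with teleport options and a player icon.
; On BeginPlay it applies the current floor plan through a dynamic material, then spawns teleporter options as child actors at map-scaled positions, plus a grid of main-floor options.
; Each tick it remaps the owning VR pawn's camera position and yaw onto the map to update the icon.
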(event `/Game/ArchVisVR/Blueprints/ArchVis_Interface.Pickup`
  (params (AttachTo :type "SceneComponent Object Reference"))
  ;[1 1 1] Pickup and drop tablet
  (`SceneComponent.K2_AttachToComponent` (`self.K2_GetRootComponent`) AttachTo "None" "KeepWorld" "KeepWorld" "KeepWorld" true))

(event `/Game/ArchVisVR/Blueprints/ArchVis_Interface.Drop`
  ;[1 1 1] Pickup and drop tablet
  (`self.K2_DetachFromActor` "KeepWorld" "KeepWorld" "KeepWorld"))

(event `self.ReceiveBeginPlay`
  (`self.GetFloorInfo`)
  (bind _returnvalue (`PrimitiveComponent.CreateDynamicMaterialInstance` (`self.Map`) 0 "/Game/ArchVisVR/Materials/MI_FloorMap.MI_FloorMap" "None"))
  (`MaterialInstanceDynamic.SetTextureParameterValue` _returnvalue "FloorMap" (`.FloorPlan_2_3DB1777D43B08E4BBF9C24A5834BD3F4` (break `/Game/ArchVisVR/Blueprints/Option/OptionType/ArchVisVR_FloorOption` (`self.CurrentFloorInfo`))))
  (`PrimitiveComponent.SetMaterial` (`self.Map`) 0 _returnvalue)
  (`self.SpawnFloorTeleporter`)
  (`self.SpawnMainFloorTeleporter`))

(event `self.ReceiveTick`
  (params (DeltaSeconds :type "Float (single-precision)"))
  (`self.UpdatePlayerIcon`))

(fn `GetFloorInfo`
  (bind _outactors (`GameplayStatics.GetAllActorsOfClass` null))
  (if (> (`KismetArrayLibrary.Array_Length` _outactors) 0)
    (set `self.CurrentFloorInfo` (struct))))

(fn `SpawnFloorTeleporter`
  (bind (_returnvalue_x _returnvalue_y) (`KismetMathLibrary.BreakVector` (`self.K2_GetActorLocation`)))
  (bind _map (`self.Map`))
  (bind (_floorplan _teleporterlocations _floorscale) (break `/Game/ArchVisVR/Blueprints/Option/OptionType/ArchVisVR_FloorOption` (`self.CurrentFloorInfo`)))
  (bind (_relativelocation_x _relativelocation_y _relativelocation_z) (`KismetMathLibrary.BreakVector` (`SceneComponent.RelativeLocation` _map)))
  (bind _relativescale3d_x (`KismetMathLibrary.BreakVector` (`SceneComponent.RelativeScale3D` _map)))
  (bind _returnvalue (* _floorscale 2048.0))
  (bind _returnvalue_2 (* _relativescale3d_x 2048.0))
  (for _array_element _teleporterlocations
    (bind (_returnvalue_x_2 _returnvalue_y_2) (`KismetMathLibrary.BreakVector` (`self.K2_GetActorLocation` _array_element)))
    (`self.SpawnTeleportOption` _array_element (* (`KismetMathLibrary.MapRangeClamped` _returnvalue_x_2 _returnvalue_x (+ _returnvalue_x _returnvalue) 0.0 1.0) (+ _relativelocation_y _returnvalue_2)) (* (`KismetMathLibrary.MapRangeClamped` _returnvalue_y_2 _returnvalue_y (- _returnvalue_y _returnvalue) 0.0 1.0) (+ _relativelocation_z _returnvalue_2)))))

(fn `SpawnMainFloorTeleporter`
  (`/Engine/EditorBlueprintResources/StandardMacros.IsValid` "/Game/ArchVisVR/Blueprints/Player/ArchVis_VRPawn_BP.ArchVis_VRPawn_BP"
    (:`Is Valid`
      (for (_array_element _array_index) _
        (if (== (mod _array_index (`self.MainFloorPerRaw`)) 0)
          (set `self.MainFloorUpHelper` (+ (`self.MainFloorUpHelper`) 1))
          (set `self.MainFloorRightHelper` 1))
        (`self.SpawnTeleportOption` _array_element (* (`self.MainFloorRightHelper`) 4.0) (* (`self.MainFloorUpHelper`) 3.0))
        (set `self.MainFloorRightHelper` (+ (`self.MainFloorRightHelper`) 1))))))

(fn `SpawnTeleportOption`
  (params (NewTeleporter :type "/Game/ArchVisVR/Blueprints/Actor/ArchVisVR_Teleporter Object Reference") (ForwardOffset :type "Float (double-precision)") (UpOffset :type "Float (double-precision)"))
  (bind _vectorhelper (`self.VectorHelper`))
  (bind _returnvalue (`AddComponent|NODE_AddChildActorComponent-3` :`bManualAttachment` true :`RelativeTransform` (`self.GetTransform`)))
  (`SceneComponent.K2_AttachToComponent` _returnvalue (`self.Map`) "None" "KeepWorld" "KeepWorld" "KeepWorld" true)
  (`KismetArrayLibrary.Array_Add` (`self.TeleporterOptions`) _returnvalue)
  (bind _astablet_teleporter_option_bp (cast `/Game/ArchVisVR/Blueprints/Option/TabletTeleporterOption_BP` (`ChildActorComponent.ChildActor` _returnvalue)))
  (`/Game/ArchVisVR/Blueprints/Option/TabletTeleporterOption_BP.InitializeOption` _astablet_teleporter_option_bp (`self.GetTransform` NewTeleporter) (struct))
  (`SceneComponent.K2_SetWorldLocation` _returnvalue (`SceneComponent.K2_GetComponentLocation` (`self.Map`)) false false)
  (`SceneComponent.K2_AddWorldOffset` _returnvalue (+ (* (`SceneComponent.GetForwardVector` _vectorhelper) ForwardOffset) (* (`SceneComponent.GetUpVector` _vectorhelper) UpOffset)) false false))

(fn `UpdatePlayerIcon`
  (bind (_returnvalue_x _returnvalue_y) (`KismetMathLibrary.BreakVector` (`self.K2_GetActorLocation`)))
  (bind _vectorhelper (`self.VectorHelper`))
  (bind _map (`self.Map`))
  (bind _playericon (`self.PlayerIcon`))
  (bind (_relativelocation_x _relativelocation_y _relativelocation_z) (`KismetMathLibrary.BreakVector` (`SceneComponent.RelativeLocation` _map)))
  (bind _relativescale3d_x (`KismetMathLibrary.BreakVector` (`SceneComponent.RelativeScale3D` _map)))
  (bind _returnvalue (* (`.FloorScale_28_63305A2C434FA3858BD34EB94D921D85` (break `/Game/ArchVisVR/Blueprints/Option/OptionType/ArchVisVR_FloorOption` (`self.CurrentFloorInfo`))) 2048.0))
  (bind _returnvalue_2 (* _relativescale3d_x 2048.0))
  (bind _asarch_vis_vrpawn_bp (cast `/Game/ArchVisVR/Blueprints/Player/ArchVis_VRPawn_BP` (`self.GetOwner`)))
  (bind _camera (`/Game/ArchVisVR/Blueprints/Player/ArchVis_VRPawn_BP.Camera` _asarch_vis_vrpawn_bp))
  (bind (_returnvalue_x_2 _returnvalue_y_2) (`KismetMathLibrary.BreakVector` (`SceneComponent.K2_GetComponentLocation` _camera)))
  (`SceneComponent.K2_SetWorldLocation` _playericon (+ (`SceneComponent.K2_GetComponentLocation` (`self.Map`)) (+ (* (`SceneComponent.GetForwardVector` _vectorhelper) (* (`KismetMathLibrary.MapRangeClamped` _returnvalue_x_2 _returnvalue_x (+ _returnvalue_x _returnvalue) 0.0 1.0) (+ _relativelocation_y _returnvalue_2))) (* (`SceneComponent.GetUpVector` _vectorhelper) (* (`KismetMathLibrary.MapRangeClamped` _returnvalue_y_2 _returnvalue_y (- _returnvalue_y _returnvalue) 0.0 1.0) (+ _relativelocation_z _returnvalue_2))))) false false)
  (`SceneComponent.K2_SetRelativeRotation` _playericon (`KismetMathLibrary.MakeRotator` (.yaw (`SceneComponent.K2_GetComponentRotation` _camera))) false false))

(fn `UserConstructionScript`)