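; Base actor for ArchVis VR objects whose color, pattern, decal and mesh can be swapped through in-world option menus.
; The motion controller opens the menus, spawning one option handler per active type at the pawn's handler anchors and filling it from the option lists.
; Apply functions use dynamic material instances, mirroring color and pattern onto related meshes, and offset new meshes from the initial transform.
; Decals follow a projector, scaled by distance.
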(event `self.ReceiveBeginPlay`
  (bind _mesh (`self.Mesh`))
  (bind _decalactor (`self.DecalActor`))
  ;[1 1 1] To Activate and Unhide decal if decal is one of active options
  (for _array_element (`self.ActiveOptions`)
    (if (`|EnumEquality` _array_element "NewEnumerator2")
      (`SceneComponent.SetVisibility` _decalactor true false)
      (`SceneComponent.SetHiddenInGame` _decalactor false false)
      (break)))
  ;[1 1 1] Save initial location & rotation to add offset later if we need
  (set `self.InitialLocation` (`SceneComponent.K2_GetComponentLocation` _mesh))
  (set `self.InitialRotation` (`SceneComponent.K2_GetComponentRotation` _mesh)))

(event `/Game/ArchVisVR/Blueprints/ArchVis_Interface.OpenArchVisOptions`
  ;[1 1 1] This will call from Motion controller to spawn available options
  (`self.SpawnHandlers`)
  (`self.AddOptionsToHandlers`))

(event `/Game/ArchVisVR/Blueprints/ArchVis_Interface.CloseArchVisOptions`
  ;[1 1 1] This will call from Motion controller to close and destroy options
  (`self.CloseOptions`))

(fn `AddOptionsToHandlers`
  (bind _colorhandler (`self.ColorHandler`))
  (bind _decalhandler (`self.DecalHandler`))
  (bind _patternhandler (`self.PatternHandler`))
  (bind _meshhandler (`self.MeshHandler`))
  ;[1 1 1] Add options from list to each handler
  (for _array_element (`self.ActiveOptions`)
    (switch `/Game/ArchVisVR/Blueprints/Option/OptionType/ArchVisVR_Options` _array_element
      (:`NewEnumerator0`
        (`/Engine/EditorBlueprintResources/StandardMacros.IsValid` (`self.ColorHandler`)
          (:`Is Valid`
            (for _array_element_2 (`self.ColorOptions`)
              (`/Game/ArchVisVR/Blueprints/Option/OptionHandler_BP.SpawnOptions` :`self` _colorhandler :`NewColorInfo` _array_element_2 :`NewUIStyle` (`self.ColorUI`)))
            (`/Game/ArchVisVR/Blueprints/Option/OptionHandler_BP.SetOptionLocationAndRotation` _colorhandler))))
      (:`NewEnumerator1`
        (`/Engine/EditorBlueprintResources/StandardMacros.IsValid` (`self.PatternHandler`)
          (:`Is Valid`
            (for _array_element_3 (`self.PatternOptions`)
              (`/Game/ArchVisVR/Blueprints/Option/OptionHandler_BP.SpawnOptions` :`self` _patternhandler :`NewPatternInfo` _array_element_3 :`NewUIStyle` (`self.PatternUI`)))
            (`/Game/ArchVisVR/Blueprints/Option/OptionHandler_BP.SetOptionLocationAndRotation` _patternhandler))))
      (:`NewEnumerator2`
        (`/Engine/EditorBlueprintResources/StandardMacros.IsValid` (`self.DecalHandler`)
          (:`Is Valid`
            (for _array_element_4 (`self.DecalOptions`)
              (`/Game/ArchVisVR/Blueprints/Option/OptionHandler_BP.SpawnOptions` :`self` _decalhandler :`NewDecalInfo` _array_element_4 :`NewUIStyle` (`self.DecalUI`)))
            (`/Game/ArchVisVR/Blueprints/Option/OptionHandler_BP.SetOptionLocationAndRotation` _decalhandler))))
      (:`NewEnumerator3`
        (`/Engine/EditorBlueprintResources/StandardMacros.IsValid` (`self.MeshHandler`)
          (:`Is Valid`
            (for _array_element_5 (`self.MeshOptions`)
              (`/Game/ArchVisVR/Blueprints/Option/OptionHandler_BP.SpawnOptions` :`self` _meshhandler :`NewMeshInfo` _array_element_5 :`NewUIStyle` (`self.MeshUI`)))
            (`/Game/ArchVisVR/Blueprints/Option/OptionHandler_BP.SetOptionLocationAndRotation` _meshhandler)))))))

(fn `ApplyNewColor`
  (params (NewInfo :type "/Game/ArchVisVR/Blueprints/Option/OptionType/ArchVisVR_ColorOption Structure"))
  (bind (_color _meshindex) (break `/Game/ArchVisVR/Blueprints/Option/OptionType/ArchVisVR_ColorOption` NewInfo))
  (`|ExecutionSequence`
    (:`then_0`
      ;[1 1 1] Apply new color info to desired mesh index (MatID)
      (`/Engine/EditorBlueprintResources/StandardMacros.IsValid` (`self.StaticMesh`)
        (:`Is Valid`
          (`/Engine/EditorBlueprintResources/StandardMacros.IsValid` (`self.MatInst`)
            (:`Is Valid`
              _)
            (:`Is Not Valid`
              (`self.CreateMatInst` _meshindex)))
          (`MaterialInstanceDynamic.SetVectorParameterValue` (`self.MatInst`) "Color" _color))))
    (:`then_1`
      (if (> (`KismetArrayLibrary.Array_Length` (`self.RelatedMeshes`)) (`KismetArrayLibrary.Array_Length` (`self.RelatedMatInst`)))
        (`self.CreateMatInst` 0))
      ;[1 1 1] Check for related meshes
      (for _array_element (`self.RelatedMatInst`)
        (`MaterialInstanceDynamic.SetVectorParameterValue` _array_element "Color" _color)))))

(fn `ApplyNewDecal`
  (params (NewInfo :type "/Game/ArchVisVR/Blueprints/Option/OptionType/ArchVisVR_DecalOption Structure"))
  (bind (_decalbasetexture _decalmaterialinstance _minsize _maxsize) (break `/Game/ArchVisVR/Blueprints/Option/OptionType/ArchVisVR_DecalOption` NewInfo))
  ;[1 1 1] Set the Min/Max decal size and new decal material
  (`DecalComponent.SetDecalMaterial` (`self.DecalActor`) _decalmaterialinstance)
  (set `self.MinDecalSize` _minsize)
  (set `self.MaxDecalSize` _maxsize))

(fn `ApplyNewMesh`
  (params (NewInfo :type "/Game/ArchVisVR/Blueprints/Option/OptionType/ArchVisVR_MeshOption Structure"))
  (bind (_picture _mesh _meshtransofrm) (break `/Game/ArchVisVR/Blueprints/Option/OptionType/ArchVisVR_MeshOption` NewInfo))
  (bind (_initialrotation_roll _initialrotation_pitch _initialrotation_yaw) (`KismetMathLibrary.BreakRotator` (`self.InitialRotation`)))
  (bind _mesh_2 (`self.Mesh`))
  ;[1 1 1] Set Mesh info: The new static Mesh, Scale, Offset Location & Offset Rotation
  (`StaticMeshComponent.SetStaticMesh` _mesh_2 _mesh)
  (`SceneComponent.SetWorldScale3D` _mesh_2 (.scale _meshtransofrm))
  (`SceneComponent.K2_SetWorldLocation` _mesh_2 (+ (.location _meshtransofrm) (`self.InitialLocation`)) false false)
  (`SceneComponent.K2_SetWorldRotation` _mesh_2 (`KismetMathLibrary.MakeRotator` (+ (.roll (.rotation _meshtransofrm)) _initialrotation_roll) (+ (.pitch (.rotation _meshtransofrm)) _initialrotation_pitch) (+ (.yaw (.rotation _meshtransofrm)) _initialrotation_yaw)) false false))

(fn `ApplyNewPattern`
  (params (NewInfo :type "/Game/ArchVisVR/Blueprints/Option/OptionType/ArchVisVR_PatternOption Structure"))
  (bind (_basetexture _patternmaterialinstance _meshindex) (break `/Game/ArchVisVR/Blueprints/Option/OptionType/ArchVisVR_PatternOption` NewInfo))
  ;[1 1 1] Apply new pattern (material) info to the desired Mesh Index (MatID)
  (bind _returnvalue (`PrimitiveComponent.CreateDynamicMaterialInstance` (`self.Mesh`) _meshindex _patternmaterialinstance "None"))
  (bind _output_get (set `self.MatInst` _returnvalue))
  (`PrimitiveComponent.SetMaterial` (`self.Mesh`) _meshindex _output_get)
  (`KismetArrayLibrary.Array_Clear` (`self.RelatedMatInst`))
  (for _array_element (`self.RelatedMeshes`)
    (bind _staticmeshcomponent (`StaticMeshActor.StaticMeshComponent` _array_element))
    (bind _returnvalue_2 (`PrimitiveComponent.CreateDynamicMaterialInstance` _staticmeshcomponent 0 _patternmaterialinstance "None"))
    (`PrimitiveComponent.SetMaterial` _staticmeshcomponent 0 _returnvalue_2)
    (`KismetArrayLibrary.Array_AddUnique` (`self.RelatedMatInst`) _returnvalue_2)))

(fn `CloseOptions`
  (bind _colorhandler (`self.ColorHandler`))
  (bind _decalhandler (`self.DecalHandler`))
  (bind _patternhandler (`self.PatternHandler`))
  (bind _meshhandler (`self.MeshHandler`))
  ;[1 1 1] Call closing function for each avaiable handler
  (`|ExecutionSequence`
    (:`then_0`
      (`/Engine/EditorBlueprintResources/StandardMacros.IsValid` _colorhandler
        (:`Is Valid`
          (`/Game/ArchVisVR/Blueprints/Option/OptionHandler_BP.CloseOptions` _colorhandler)
          (set `self.ColorHandler` null))))
    (:`then_1`
      (`/Engine/EditorBlueprintResources/StandardMacros.IsValid` _decalhandler
        (:`Is Valid`
          (`/Game/ArchVisVR/Blueprints/Option/OptionHandler_BP.CloseOptions` _decalhandler)
          (set `self.DecalHandler` null))))
    (:`then_2`
      (`/Engine/EditorBlueprintResources/StandardMacros.IsValid` _patternhandler
        (:`Is Valid`
          (`/Game/ArchVisVR/Blueprints/Option/OptionHandler_BP.CloseOptions` _patternhandler)
          (set `self.PatternHandler` null))))
    (:`then_3`
      (`/Engine/EditorBlueprintResources/StandardMacros.IsValid` _meshhandler
        (:`Is Valid`
          (`/Game/ArchVisVR/Blueprints/Option/OptionHandler_BP.CloseOptions` _meshhandler)
          (set `self.MeshHandler` null))))))

(fn `CreateMatInst`
  (params (NewIndex :type Integer))
  (bind _mesh (`self.Mesh`))
  (`|ExecutionSequence`
    (:`then_0`
      ;[1 1 1] Create material instance for desired mesh index and also for related meshes
      (`/Engine/EditorBlueprintResources/StandardMacros.IsValid` (`self.StaticMesh`)
        (:`Is Valid`
          (`/Engine/EditorBlueprintResources/StandardMacros.IsValid` (`self.MatInst`)
            (:`Is Not Valid`
              (bind _returnvalue (`PrimitiveComponent.CreateDynamicMaterialInstance` _mesh NewIndex (`PrimitiveComponent.GetMaterial` _mesh NewIndex) "None"))
              (set `self.MatInst` _returnvalue))))))
    (:`then_1`
      ;[1 1 1] Creat MaterialInstance for related meshes and add it to array
      (if (> (`KismetArrayLibrary.Array_Length` (`self.RelatedMeshes`)) (`KismetArrayLibrary.Array_Length` (`self.RelatedMatInst`)))
        (for _array_element (`self.RelatedMeshes`)
          (bind _staticmeshcomponent (`StaticMeshActor.StaticMeshComponent` _array_element))
          (bind _returnvalue_2 (`PrimitiveComponent.CreateDynamicMaterialInstance` _staticmeshcomponent 0 (`PrimitiveComponent.GetMaterial` _staticmeshcomponent 0) "None"))
          (`KismetArrayLibrary.Array_AddUnique` (`self.RelatedMatInst`) _returnvalue_2))))))

(fn `SpawnHandlers`
  ;[1 1 1] Spawn handler for each active option
  (for (_array_element _array_index) (`self.ActiveOptions`)
    ;;[1 1 1] Find  transforms to spawn handlers
    (bind _asarch_vis_vrpawn_bp (cast `/Game/ArchVisVR/Blueprints/Player/ArchVis_VRPawn_BP` (`GameplayStatics.GetPlayerPawn` 0)))
    (switch `int` _array_index
      (:`0`
        (set `self.SpawnTransform` (`SceneComponent.K2_GetComponentToWorld` (`/Game/ArchVisVR/Blueprints/Player/ArchVis_VRPawn_BP.Handler_1` _asarch_vis_vrpawn_bp))))
      (:`1`
        (set `self.SpawnTransform` (`SceneComponent.K2_GetComponentToWorld` (`/Game/ArchVisVR/Blueprints/Player/ArchVis_VRPawn_BP.Handler_2` _asarch_vis_vrpawn_bp))))
      (:`2`
        (set `self.SpawnTransform` (`SceneComponent.K2_GetComponentToWorld` (`/Game/ArchVisVR/Blueprints/Player/ArchVis_VRPawn_BP.Handler_3` _asarch_vis_vrpawn_bp))))
      (:`3`
        (set `self.SpawnTransform` (`SceneComponent.K2_GetComponentToWorld` (`/Game/ArchVisVR/Blueprints/Player/ArchVis_VRPawn_BP.Handler_4` _asarch_vis_vrpawn_bp)))))
    ;;[1 1 1] Spawn and set variables for handlers
    (bind _returnvalue (`|SpawnActorFromClass` "/Game/ArchVisVR/Blueprints/Option/OptionHandler_BP.OptionHandler_BP_C" (`self.SpawnTransform`) "Undefined" "OverrideRootScale" self _array_element null))
    (switch `/Game/ArchVisVR/Blueprints/Option/OptionType/ArchVisVR_Options` _array_element
      (:`NewEnumerator0`
        (set `self.ColorHandler` _returnvalue))
      (:`NewEnumerator1`
        (set `self.PatternHandler` _returnvalue))
      (:`NewEnumerator2`
        (set `self.DecalHandler` _returnvalue))
      (:`NewEnumerator3`
        (set `self.MeshHandler` _returnvalue)))))

(fn `UpdateDecal`
  (params (NewProjectorLocation :type "Vector Structure") (NewDistance :type "Float (double-precision)") (NewDecalLocation :type "Vector Structure") (NewProjectorRotation :type "Rotator Structure"))
  (bind _decalactor (`self.DecalActor`))
  ;[1 1 1] Update Decal size location from decal projector
  ;;[1 1 1] Set Location
  (`SceneComponent.K2_SetWorldLocationAndRotation` (`self.DecalProjectorLocation`) NewProjectorLocation (`KismetMathLibrary.MakeRotator` (.roll NewProjectorRotation) (.pitch (`self.K2_GetActorRotation`)) (.yaw (`self.K2_GetActorRotation`))) false false)
  (`SceneComponent.K2_SetWorldLocation` _decalactor NewDecalLocation false true)
  ;;[1 1 1] Size dependson distance
  (`SceneComponent.SetWorldScale3D` _decalactor (`KismetMathLibrary.VLerp` (1.0 0.1 0.1) (1.0 1.0 1.0) (`KismetMathLibrary.MapRangeClamped` NewDistance (`self.MinDecalSize`) (`self.MaxDecalSize`) 0.0 1.0))))

(fn `UserConstructionScript`
  (`StaticMeshComponent.SetStaticMesh` (`self.Mesh`) (`self.StaticMesh`))
  (for _array_element (`self.OptionTypes`)
    (`KismetArrayLibrary.Array_AddUnique` (`self.ActiveOptions`) _array_element))
  (if (`self.Pickupable`)
    _))