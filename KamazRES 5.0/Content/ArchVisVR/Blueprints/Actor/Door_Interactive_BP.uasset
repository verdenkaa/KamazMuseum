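; VR door actor that a motion controller grabs at its handle and moves by rotating or sliding along X, Y or Z.
; DoorAttached finds the overlapping controller and stores its grab offset; Drop or leaving the handle collision releases it.
; While grabbed, Tick follows the controller, clamping slides between the construction-time origin and a mirrorable MaxOffset.
; Rotation uses clamped look-at yaw; a distance-based alternative remains unconnected, marked not working.
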(event `self.ReceiveTick`
  (params (DeltaSeconds :type "Float (single-precision)"))
  (bind _returnvalue (`self.K2_GetActorLocation`))
  (bind _mcontroller (`self.MController`))
  (bind _returnvalue_2 (`SceneComponent.K2_GetComponentLocation` (`/Game/ArchVisVR/Blueprints/Player/ArchVis_MotionController_BP.MotionController` _mcontroller)))
  ;[1 1 1] Move door
  (if (`self.bDoorGrabed`)
    (`/Engine/EditorBlueprintResources/StandardMacros.IsValid` _mcontroller
      (:`Is Valid`
        (switch `/Game/ArchVisVR/Blueprints/Option/OptionType/ArchVisVR_DoorType` (`self.DoorType`)
          (:`NewEnumerator0`
            (`self.RotatingDoor` _returnvalue_2))
          (:`NewEnumerator1`
            (`self.SlideInX` _returnvalue_2 _returnvalue))
          (:`NewEnumerator2`
            (`self.SlideInY` _returnvalue_2 _returnvalue))
          (:`NewEnumerator3`
            (`self.SlideInZ` _returnvalue_2 _returnvalue))))
      (:`Is Not Valid`
        (set `self.bDoorGrabed` false)))))

(event `/Game/ArchVisVR/Blueprints/ArchVis_Interface.DoorAttached`
  (params (AttachTo :type "SceneComponent Object Reference"))
  (bind _mcontroller (`self.MController`))
  (bind _returnvalue (`SceneComponent.K2_GetComponentLocation` (`/Game/ArchVisVR/Blueprints/Player/ArchVis_MotionController_BP.MotionController` _mcontroller)))
  ;[1 1 1] When dor grabbed by hands this function will set default handler location
  (for _array_element (`PrimitiveComponent.GetOverlappingActors` (`self.HandlerCollision`) null)
    (bind _asarch_vis_motion_controller_bp (cast `/Game/ArchVisVR/Blueprints/Player/ArchVis_MotionController_BP` _array_element))
    (set `self.MController` _asarch_vis_motion_controller_bp)
    (set `self.bDoorGrabed` true)
    (break))
  (if (`self.bDoorGrabed`)
    (`/Engine/EditorBlueprintResources/StandardMacros.IsValid` _mcontroller
      (:`Is Valid`
        (switch `/Game/ArchVisVR/Blueprints/Option/OptionType/ArchVisVR_DoorType` (`self.DoorType`)
          (:`NewEnumerator0`
            (bind _output_get (set `self.InitialHandlerLocation` (`SceneComponent.K2_GetComponentLocation` (`self.HandlerCollision`))))
            (set `self.Distance` (`KismetMathLibrary.VSize` (- _returnvalue _output_get))))
          (:`NewEnumerator1`
            (set `self.Distance` (.x (- _returnvalue (`self.K2_GetActorLocation`)))))
          (:`NewEnumerator2`
            (set `self.Distance` (.y (- _returnvalue (`self.K2_GetActorLocation`)))))
          (:`NewEnumerator3`
            (set `self.Distance` (.z (- _returnvalue (`self.K2_GetActorLocation`))))))))))

(event `/Game/ArchVisVR/Blueprints/ArchVis_Interface.Drop`
  ;[1 1 1] Event for toching handler by hands
  (set `self.bDoorGrabed` false :!label _label)
  (set `self.MController` (stale `self.HandlerCollision.OnComponentEndOverlap` _asarch_vis_motion_controller_bp))
  (set `self.bHandlerTouch` false))

(event `self.HandlerCollision.OnComponentEndOverlap`
  (params (OverlappedComponent :type "PrimitiveComponent Object Reference") (OtherActor :type "Actor Object Reference") (OtherComp :type "PrimitiveComponent Object Reference") (OtherBodyIndex :type Integer))
  ;[1 1 1] Event for toching handler by hands
  (bind _asarch_vis_motion_controller_bp (cast `/Game/ArchVisVR/Blueprints/Player/ArchVis_MotionController_BP` OtherActor))
  (goto _label))

(event `self.HandlerCollision.OnComponentBeginOverlap`
  (params (OverlappedComponent :type "PrimitiveComponent Object Reference") (OtherActor :type "Actor Object Reference") (OtherComp :type "PrimitiveComponent Object Reference") (OtherBodyIndex :type Integer) (bFromSweep :type Boolean) (SweepResult :type "HitResult Structure (by ref)"))
  ;[1 1 1] Event for toching handler by hands
  (set `self.bHandlerTouch` (`.bSuccess` (cast `/Game/ArchVisVR/Blueprints/Player/ArchVis_MotionController_BP` OtherActor :!pure true))))

(fn `RotatingDoor`
  (params (ControllerLocation :type "Vector Structure"))
  (bind (_returnvalue_roll _returnvalue_pitch) (`KismetMathLibrary.BreakRotator` (`self.K2_GetActorRotation`)))
  (bind (_returnvalue_roll_2 _returnvalue_pitch_2 _returnvalue_yaw) (`KismetMathLibrary.BreakRotator` (`KismetMathLibrary.FindLookAtRotation` ControllerLocation (`self.K2_GetActorLocation`))))
  (`self.K2_SetActorRotation` (`KismetMathLibrary.MakeRotator` _returnvalue_roll _returnvalue_pitch (`KismetMathLibrary.FClamp` _returnvalue_yaw (`self.MinRotation`) (`self.MaxRotation`)))))

(fn `SlideInX`
  (params (ControllerLocation :type "Vector Structure") (DoorLocation :type "Vector Structure"))
  (locals (DefaultY :type "Float (double-precision)") (DefaultZ :type "Float (double-precision)"))
  (bind _x (.x (`self.WorldOrigin`)))
  (bind _returnvalue (+ _x (`self.MaxOffset`)))
  ;[1 1 1] Set door location in X Axsis limited to default location and max offset
  (set `local.DefaultY` (.y DoorLocation))
  (set `local.DefaultZ` (.z DoorLocation))
  (if (`self.bIsMirror`)
    (`self.K2_SetActorLocation` (`KismetMathLibrary.MakeVector` (`KismetMathLibrary.FClamp` (+ (* (`self.Distance`) -1.0) (.x ControllerLocation)) _x _returnvalue) (`local.DefaultY`) (`local.DefaultZ`)))
    (else
      (`self.K2_SetActorLocation` (`KismetMathLibrary.MakeVector` (`KismetMathLibrary.FClamp` (- (.x ControllerLocation) (`self.Distance`)) _returnvalue _x) (`local.DefaultY`) (`local.DefaultZ`))))))

(fn `SlideInY`
  (params (ControllerLocation :type "Vector Structure") (DoorLocation :type "Vector Structure"))
  (locals (DefaultX :type "Float (double-precision)") (DefaultZ :type "Float (double-precision)"))
  (bind _y (.y (`self.WorldOrigin`)))
  (bind _returnvalue (- _y (`self.MaxOffset`)))
  ;[1 1 1] Set door location in Y Axsis limited to default location and max offset
  (set `local.DefaultX` (.x DoorLocation))
  (set `local.DefaultZ` (.z DoorLocation))
  (if (`self.bIsMirror`)
    (`self.K2_SetActorLocation` (`KismetMathLibrary.MakeVector` (`local.DefaultX`) (`KismetMathLibrary.FClamp` (+ (* (`self.Distance`) -1.0) (.y ControllerLocation)) _returnvalue _y) (`local.DefaultZ`)))
    (else
      (`self.K2_SetActorLocation` (`KismetMathLibrary.MakeVector` (`local.DefaultX`) (`KismetMathLibrary.FClamp` (- (.y ControllerLocation) (`self.Distance`)) _y _returnvalue) (`local.DefaultZ`))))))

(fn `SlideInZ`
  (params (ControllerLocation :type "Vector Structure") (DoorLocation :type "Vector Structure"))
  (locals (DefaultX :type "Float (double-precision)") (DefaultY :type "Float (double-precision)"))
  (bind _maxoffset (`self.MaxOffset`))
  (bind _z (.z (`self.WorldOrigin`)))
  ;[1 1 1] Set door location in Z Axsis limited to default location and max offset
  (set `local.DefaultX` (.x DoorLocation))
  (set `local.DefaultY` (.y DoorLocation))
  (if (`self.bIsMirror`)
    (`self.K2_SetActorLocation` (`KismetMathLibrary.MakeVector` (`local.DefaultX`) (`local.DefaultY`) (`KismetMathLibrary.FClamp` (+ (* (`self.Distance`) -1.0) (.z ControllerLocation)) _z (+ _z _maxoffset))))
    (else
      (`self.K2_SetActorLocation` (`KismetMathLibrary.MakeVector` (`local.DefaultX`) (`local.DefaultY`) (`KismetMathLibrary.FClamp` (- (.z ControllerLocation) (`self.Distance`)) _z (- _z _maxoffset)))))))

(fn `UserConstructionScript`
  (`parent.UserConstructionScript`)
  (set `self.WorldOrigin` (`self.K2_GetActorLocation`)))